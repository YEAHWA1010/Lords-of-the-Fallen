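; BP_Sound3D is a trigger actor that calls a positional sound playback at its own location when BP_Player_ overlaps its Box.
; The overlap sets a non-looping half-second timer for PlaySound, then waits PlayTime before clearing TimerHandle.
; As written, Play is only ever set false, TimerHandle is set to None, and no sound asset is specified.
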(event `self.Box.OnComponentBeginOverlap`
  (params (OverlappedComponent :type "PrimitiveComponent Object Reference") (OtherActor :type "Actor Object Reference") (OtherComp :type "PrimitiveComponent Object Reference") (OtherBodyIndex :type Integer) (bFromSweep :type Boolean) (SweepResult :type "HitResult Structure (by ref)"))
  (cast `/Game/Main/BluePrints/BP_Player_` OtherActor)
  (if (not (`self.Play`))
    (set `self.Play` false)
    (`KismetSystemLibrary.K2_SetTimerDelegate` (delegate `PlaySound`) 0.5) ; 이벤트가 일정 시간마다\n연결된 함수가 일정시간마다 호출
    (set `self.TimerHandle` (struct)) ; 저장해놔야 이 타이머만 지울 수 있음
    (`KismetSystemLibrary.Delay` (`self.PlayTime`))
    (`KismetSystemLibrary.K2_ClearAndInvalidateTimerHandle` (`self.TimerHandle`))
    (set `self.Play` false)))

(event `PlaySound`
  (`GameplayStatics.PlaySoundAtLocation` null (`self.K2_GetActorLocation`) (struct) 1.0 1.0 0.0 null null null null))

(fn `UserConstructionScript`)