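; Base weapon Blueprint with empty hooks for selection, collision toggling and Attack, apparently meant for child weapons to override.
; State, combat type and move permission live on the owner, accessed through BPI_Weapon messages.
; CanAttack requires the owner's combat type to match this weapon's and its state to be the first enum entry, which EndAttack restores.
; SendDamage damages non-owner Characters using the owner's current weapon Power.
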(event `SetOnCollision`)

(event `SetOffCollsion`)

(event `OnSelected`)

(event `OffSelected`)

(fn `Attack`
  ;[1 1 1] 가상함수
)

(fn `CanAttack`
  (returns (Result :type Boolean))
  (return (and (`|EnumEquality` (`self.GetCombat`) (`self.CombatType`)) (`|EnumEquality` (`self.GetState`) "NewEnumerator0"))))

(fn `End Attack`
  (`self.SetState` "NewEnumerator0"))

(fn `GetCanMove`
  (returns (CanMove :type Boolean))
  (bind _returnvalue (`self.GetOwner`))
  (if (`KismetSystemLibrary.DoesImplementInterface` _returnvalue "/Game/Main/BPI_Weapon.BPI_Weapon_C")
    (bind _canmove (message `/Game/Main/BPI_Weapon.GetWeapon_CanMove` _returnvalue))
    (return _canmove)))

(fn `GetCombat`
  (returns (Combat :type "/Game/Main/Character/ECombatType Enum"))
  (bind _returnvalue (`self.GetOwner`))
  (if (`KismetSystemLibrary.DoesImplementInterface` _returnvalue "/Game/Main/BPI_Weapon.BPI_Weapon_C")
    (bind _combat (message `/Game/Main/BPI_Weapon.GetWeapon_Combat` _returnvalue))
    (return _combat)))

(fn `GetState`
  (returns (State :type "/Game/Main/Character/Boss/AI/Pieta_Sword/EStateType Enum"))
  (bind _returnvalue (`self.GetOwner`))
  (if (`KismetSystemLibrary.DoesImplementInterface` _returnvalue "/Game/Main/BPI_Weapon.BPI_Weapon_C")
    (bind _state_ (message `/Game/Main/BPI_Weapon.GetWeapon_State` _returnvalue))
    (return _state_)))

(fn `SendDamage`
  (params (OtherActor :type "Actor Object Reference"))
  (bind _returnvalue (`self.GetOwner`))
  (if (!= OtherActor (`self.GetOwner`))
    (bind `_as캐릭터` (cast `Character` OtherActor))
    (bind _weapon (message `/Game/Main/BPI_Weapon.GetWeapon_Current` _returnvalue))
    (`GameplayStatics.ApplyDamage` `_as캐릭터` (`/Game/Main/BP_Weapon.Power` _weapon) (`self.GetInstigatorController` _returnvalue) _weapon)))

(fn `SetCanMove`
  (params (CanMove :type Boolean))
  (returns (Result :type Boolean))
  (bind _returnvalue (`self.GetOwner`))
  (if (`KismetSystemLibrary.DoesImplementInterface` _returnvalue "/Game/Main/BPI_Weapon.BPI_Weapon_C")
    (bind _result (message `/Game/Main/BPI_Weapon.SetWeapon_CanMove` _returnvalue CanMove))
    (return _result)))

(fn `SetCharacter`
  (params (CharacterType :type "Character Object Reference"))
  (returns (Result :type "Character Object Reference"))
  (return null))

(fn `SetCombat`
  (params (Combat :type "/Game/Main/Character/ECombatType Enum" :default "NewEnumerator0"))
  (bind _returnvalue (`self.GetOwner`))
  (if (`KismetSystemLibrary.DoesImplementInterface` _returnvalue "/Game/Main/BPI_Weapon.BPI_Weapon_C")
    (message `/Game/Main/BPI_Weapon.SetWeapon_Combat` _returnvalue Combat)))

(fn `SetState`
  (params (State :type "/Game/Main/Character/Boss/AI/Pieta_Sword/EStateType Enum" :default "NewEnumerator0"))
  (bind _returnvalue (`self.GetOwner`))
  (if (`KismetSystemLibrary.DoesImplementInterface` _returnvalue "/Game/Main/BPI_Weapon.BPI_Weapon_C")
    (message `/Game/Main/BPI_Weapon.SetWeapon_State` _returnvalue State)))

(fn `UserConstructionScript`)