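; BP_Sword is the player's melee sword weapon, handling combo attacks and hit detection.
; Attack starts a montage or, inside the combo window, queues the next one, which PlayNextCombo plays from the player's combo montages.
; It flags the final combo step to spawn a particle effect at the damaged actor's location, and EndAttack resets the chain.
; A capsule, off by default and toggled by events, sends damage on overlap.
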(event `SetWeaponCharacter`
  (params (Character :type "/Game/Main/BluePrints/BP_Player_ Object Reference"))
  ;[1 1 1] Attack Combo
  (set `self.Player` Character))

(event `self.Attack`
  ;[1 1 1] Attack Combo
  (message `/Game/Main/BPI_Weapon.SetWeapon_CanMove` self false)
  (if (`self.EnableNextCombo`)
    (`/Engine/EditorBlueprintResources/StandardMacros.IncrementInt` (`self.ComboCount`)
      (:`  `
        (set `self.ExistNextCombo` true)
        (set `self.EnableNextCombo` false)))
    (elif (`self.CanAttack`)
      (`self.SetState` "NewEnumerator5")
      (`/Game/Main/BluePrints/BP_Player_.PlayPlayerMontage` (`self.Player`)))))

(event `PlayNextCombo`
  ;[1 1 1] Attack Combo
  (if (`self.ExistNextCombo`)
    (`/Game/Main/BluePrints/BP_Player_.PlayPlayerMontage` (`self.Player`))
    (set `self.ExistNextCombo` false)
    (set `self.LastCombo` (== (- (`KismetArrayLibrary.Array_Length` (`/Game/Main/BluePrints/BP_Player_.ComboMontages` (`self.Player`))) 1) (`self.ComboCount`)))))

(event `self.End Attack`
  ;[1 1 1] Attack Combo
  (`parent.End Attack`)
  (set `self.ComboCount` 0)
  (`self.SetCanMove` true)
  (set `self.ExistNextCombo` false))

(event `CheckNextCombo`)

(event `PlayLastComboEffect`
  (params (Damager :type "Character Object Reference"))
  (if (`self.LastCombo`)
    (`GameplayStatics.SpawnEmitterAtLocation` null (`self.K2_GetActorLocation` Damager))
    (set `self.LastCombo` false)))

(event `self.ReceiveBeginPlay`
  (`self.SetOffCollsion`)
  (set `self.CombatType` "NewEnumerator0")
  (`parent.ReceiveBeginPlay`))

(event `self.Capsule.OnComponentBeginOverlap`
  (params (OverlappedComponent :type "PrimitiveComponent Object Reference") (OtherActor :type "Actor Object Reference") (OtherComp :type "PrimitiveComponent Object Reference") (OtherBodyIndex :type Integer) (bFromSweep :type Boolean) (SweepResult :type "HitResult Structure (by ref)"))
  ;[1 1 1] Damage호출
  (`self.SendDamage` OtherActor))

(event `self.SetOnCollision`
  ;[1 1 1] Collision
  (`PrimitiveComponent.SetCollisionEnabled` (`self.Capsule`) "QueryAndPhysics"))

(event `self.SetOffCollsion`
  ;[1 1 1] Collision
  (`PrimitiveComponent.SetCollisionEnabled` (`self.Capsule`) "NoCollision"))

(fn `UserConstructionScript`)