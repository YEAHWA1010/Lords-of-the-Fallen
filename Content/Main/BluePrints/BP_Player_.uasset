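; Player character Blueprint for a third-person melee game, handling movement, camera zoom, sprint, dive roll, parry and sword combat.
; BeginPlay spawns and attaches BP_Sword and loads combo montages from a data table for sword attacks.
; Lock-on sphere-traces for enemies, picks one by camera dot product, shows its cursor and turns the controller toward it each tick.
; Damage triggers hit reactions facing the attacker; death shows an ending widget, then quits.
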(event `InputAction|Run`
  (params (Key :type "Key Structure"))
  (bind _charactermovement (`self.CharacterMovement`))
  ;[1 1 1] Basic
  (:`Pressed`
    (set `CharacterMovementComponent.MaxWalkSpeed` 600.0 _charactermovement)
    (bind _result (`/Engine/EditorBlueprintResources/StandardMacros.DecrementFloat` (`self.CurrentStamina`))
      (:`  `
        (set `self.CurrentStamina` _result))))
  (:`Released`
    (set `CharacterMovementComponent.MaxWalkSpeed` 400.0 _charactermovement)))

(event `End_Attack`
  ;[1 1 1] Basic
)

(event `InputAction|Attacking`
  (params (Key :type "Key Structure"))
  ;[1 1 1] Basic
  (:`Pressed`
    (`/Engine/EditorBlueprintResources/StandardMacros.IsValid` (`self.Sword`)
      (:`Is Valid`
        (`self.Zoom`)
        (`/Game/Main/BP_Weapon.Attack` (`self.Sword`))))))

(event `InputAction|Parry`
  (params (Key :type "Key Structure"))
  ;[1 1 1] Basic
  (:`Pressed`
    (`/Engine/EditorBlueprintResources/StandardMacros.IsValid` (`self.Sword`)
      (:`Is Valid`
        (`self.PlayAnimMontage` "/Game/Main/Player_Anim/Player_Parry.Player_Parry")
        (set `self.IsParring` true)))))

(event `self.ReceiveBeginPlay`
  ;[1 1 1] Basic
  (`|ExecutionSequence`
    (:`then_0`
      (bind _returnvalue (`|SpawnActorFromClass` "/Game/Main/BluePrints/BP_Sword.BP_Sword_C" (`KismetMathLibrary.MakeTransform` (0.0 0.0 0.0)) "Undefined" "OverrideRootScale" self null)) ; 생성된 객체 넘김
      (bind _output_get (set `self.Sword` _returnvalue))
      (`self.K2_AttachToComponent` _output_get (`self.Mesh`) "Hand_Sword" "KeepRelative" "KeepRelative" "KeepRelative" true)
      (`/Game/Main/BluePrints/BP_Sword.SetWeaponCharacter` (`self.Sword`) self))
    (:`then_1`
      (bind _output_get_2 (set `self.PlayerComboTable` "/Game/Player_Combo_Table.Player_Combo_Table"))
      (bind _outrownames (`DataTableFunctionLibrary.GetDataTableRowNames` _output_get_2))
      (for _array_element _outrownames
        (bind _returnvalue_2 (`|GetDataTableRow` _output_get_2 _array_element)
          (:`then`
            (`KismetArrayLibrary.Array_Add` (`self.ComboMontages`) _returnvalue_2)))))
    (:`then_2`
      (switch `/Game/Main/Character/ECombatType` (`self.Combat`)
        (:`NewEnumerator0`
          (set `self.Weapon` (`self.Sword`)))))))

(event `InputAction|Rolling`
  (params (Key :type "Key Structure"))
  ;[1 1 1] Basic
  (:`Pressed`
    (`|ExecutionSequence`
      (:`then_0`
        (set `self.State` "NewEnumerator6")
        (set `self.bUseControllerRotationYaw` false)
        (set `CharacterMovementComponent.bOrientRotationToMovement` true (`self.CharacterMovement`)))
      (:`then_2`
        (`self.PlayAnimMontage` "/Game/Main/Player_Anim/SK_Player_Skeleton_AS_GENE_DiveRoll_HeavyFnt_2_5m_Montage.SK_Player_Skeleton_AS_GENE_DiveRoll_HeavyFnt_2_5m_Montage")))))

(event `End Rolling`
  ;[1 1 1] Basic
  (set `self.State` "NewEnumerator0")
  (set `self.bUseControllerRotationYaw` true)
  (set `CharacterMovementComponent.bOrientRotationToMovement` false (`self.CharacterMovement`)))

(event `InputAxis|MoveForward`
  (params (AxisValue :type "Float (single-precision)"))
  (bind (_returnvalue_roll _returnvalue_pitch _returnvalue_yaw) (`KismetMathLibrary.BreakRotator` (`self.GetControlRotation`)))
  ;[1 1 1] Basic
  (if (`self.CanMove`)
    (`self.AddMovementInput` (`KismetMathLibrary.Vector_Normal2D` (`KismetMathLibrary.GetForwardVector` (`KismetMathLibrary.MakeRotator` 0.0 0.0 _returnvalue_yaw))) AxisValue)))

(event `InputAxis|MoveRight`
  (params (AxisValue :type "Float (single-precision)"))
  (bind (_returnvalue_roll _returnvalue_pitch _returnvalue_yaw) (`KismetMathLibrary.BreakRotator` (`self.GetControlRotation`)))
  ;[1 1 1] Basic
  (if (`self.CanMove`)
    (`self.AddMovementInput` (`KismetMathLibrary.Vector_Normal2D` (`KismetMathLibrary.GetRightVector` (`KismetMathLibrary.MakeRotator` 0.0 0.0 _returnvalue_yaw))) AxisValue)))

(event `InputAxis|VerticalLock`
  (params (AxisValue :type "Float (single-precision)"))
  ;[1 1 1] Basic
  (`self.AddControllerPitchInput` AxisValue))

(event `InputAxis|HorizontalLock`
  (params (AxisValue :type "Float (single-precision)"))
  ;[1 1 1] Basic
  (`self.AddControllerYawInput` AxisValue))

(event `InputAxis|Zoom`
  (params (AxisValue :type "Float (single-precision)"))
  ;[1 1 1] Basic
  (set `SpringArmComponent.TargetArmLength` (`KismetMathLibrary.FClamp` (+ (* AxisValue (`self.ZoomSpeed`)) (`SpringArmComponent.TargetArmLength` (`self.SpringArm`))) 100.0 600.0) (`self.SpringArm`)))

(event `InputAction|Targeting`
  (params (Key :type "Key Structure"))
  ;[1 1 1] Targeting
  (:`Pressed`
    (if (`self.LockOnTarget`)
      (`self.EndLockOn`)
      (`self.SetTargetCursor` (`self.LockOnEnemy`))
      (else
        (`self.StartLockOn`)))))

(event `StartLockOn`
  ;[1 1 1] Targeting
  (`self.GetTraceTargets`)
  (bind _enemy (`self.GetTargetEnemy`))
  (`/Engine/EditorBlueprintResources/StandardMacros.IsValid` _enemy
    (:`Is Valid`
      (set `self.LockOnEnemy` _enemy)
      (set `self.LockOnTarget` true))))

(event `TickLockOn`
  ;[1 1 1] Targeting
  (if (`self.LockOnTarget`)
    (`/Engine/EditorBlueprintResources/StandardMacros.IsValid` (`self.LockOnEnemy`)
      (:`Is Valid`
        (`Controller.SetControlRotation` (`self.GetController`) (`KismetMathLibrary.FindLookAtRotation` (`self.K2_GetActorLocation`) (`self.K2_GetActorLocation` (`self.LockOnEnemy`)))))
      (:`Is Not Valid`
        (`self.EndLockOn`)))))

(event `EndLockOn`
  ;[1 1 1] Targeting
  (set `self.LockOnEnemy` null)
  (set `self.LockOnTarget` false))

(event `self.ReceiveTick`
  (params (DeltaSeconds :type "Float (single-precision)"))
  ;[1 1 1] Targeting
  (`self.TickLockOn`))

(event `self.ReceiveAnyDamage`
  (params (Damage :type "Float (single-precision)") (DamageType :type "DamageType Object Reference") (InstigatedBy :type "Controller Object Reference") (DamageCauser :type "Actor Object Reference"))
  (bind (_returnvalue_roll _returnvalue_pitch _returnvalue_yaw) (`KismetMathLibrary.BreakRotator` (`KismetMathLibrary.FindLookAtRotation` (`self.K2_GetActorLocation`) (`self.K2_GetActorLocation` (`self.Attacker`)))))
  ;[1 1 1] Damage
  (set `self.Causer` DamageCauser)
  (bind `_as캐릭터` (cast `Character` (`Controller.K2_GetPawn` InstigatedBy)))
  (set `self.Attacker` `_as캐릭터`)
  (bind _output_get (set `/Game/StatusComponent.Health` (- (`/Game/StatusComponent.Health` (`self.StatusComponent`)) Damage) (`self.StatusComponent`)))
  (if (<= _output_get 0.0)
    (set `self.State` "NewEnumerator17")
    (`self.PlayAnimMontage` "/Game/Main/Player_Anim/Montages/Player_FinalDeath_Montage.Player_FinalDeath_Montage")
    (`self.Zoom`)
    (`KismetSystemLibrary.Delay` 5.0)
    (bind _returnvalue (`|CreateWidget` "/Game/UMG_EndingScene.UMG_EndingScene_C"))
    (`UserWidget.AddToViewport` _returnvalue 0)
    (`GameplayStatics.PlaySound2D` "/Game/Sound/Ending_Cue.Ending_Cue" 1.0 1.0 0.0 null null)
    (`KismetSystemLibrary.Delay` 3.0)
    (`KismetSystemLibrary.QuitGame` null "Background") ; 게임 종료
    (else
      (set `self.State` "NewEnumerator2")
      (`/Game/Main/BPI_Weapon.SetWeapon_CanMove` false)
      (`self.PlayAnimMontage` "/Game/Main/Player_Anim/Montages/Player_Hitted_03_Montage.Player_Hitted_03_Montage" 2.0)
      (`self.K2_SetActorRotation` (`KismetMathLibrary.MakeRotator` _returnvalue_roll _returnvalue_pitch _returnvalue_yaw))
      (`/Game/Main/BPI_Weapon.SetWeapon_CanMove` true)
      (set `self.State` "NewEnumerator0"))))

(event `InputAction|QuitGame`
  (params (Key :type "Key Structure"))
  ;[1 1 1] Damage
  ;;[1 1 1] End
  (:`Pressed`
    (`KismetSystemLibrary.QuitGame` null "Background")))

(event `Zoom`
  ;[1 1 1] CameraControll
  (if (`|EnumEquality` (`self.State`) "NewEnumerator17")
    (set `SpringArmComponent.TargetArmLength` (`KismetMathLibrary.FClamp` (+ (* 1.0 (`self.ZoomSpeed`)) (`SpringArmComponent.TargetArmLength` (`self.SpringArm`))) 100.0 900.0) (`self.SpringArm`))
    (else
      (set `SpringArmComponent.TargetArmLength` (`KismetMathLibrary.FClamp` (+ (* 1.0 (`self.ZoomSpeed`)) (`SpringArmComponent.TargetArmLength` (`self.SpringArm`))) 100.0 800.0) (`self.SpringArm`)))))

(fn `CanAttack`
  (returns (CanAttack :type Boolean))
  (return (`|EnumEquality` (`self.State`) "NewEnumerator0")))

(fn `Die`
  (`PrimitiveComponent.SetCollisionEnabled` (`self.CapsuleComponent`) "NoCollision")
  (`self.PlayAnimMontage` "/Game/Main/Player_Anim/SK_Player_Skeleton_AS_GENE_Death_FirstDeath_Montage.SK_Player_Skeleton_AS_GENE_Death_FirstDeath_Montage" 1.0 "Start")
  (return))

(fn `GetRollDirection`
  (returns (ReturnValue :type "Rotator Structure")))

(fn `GetTargetEnemy`
  (returns (Enemy :type "/Game/Main/BluePrints/BP_Enemy Object Reference"))
  (locals (Angle :type "Float (double-precision)") (Result :type "/Game/Main/BluePrints/BP_Enemy Object Reference"))
  (for _array_element (`self.TargetEnemies`)
    (bind _returnvalue (`self.GetDotProductTo` (`GameplayStatics.GetPlayerCameraManager` 0) _array_element))
    (if (>= _returnvalue (`local.Angle`))
      (set `local.Angle` _returnvalue)
      (set `local.Result` _array_element)))
  (`self.SetTargetCursor` (`local.Result`))
  (return (`local.Result`)))

(fn `GetTraceTargets`
  (bind _returnvalue (`self.K2_GetActorLocation`))
  (bind _outhits (`KismetSystemLibrary.SphereTraceMultiForObjects` :`Start` _returnvalue :`End` _returnvalue :`Radius` (`self.LockDistance`) :`ObjectTypes` (`|MakeArray` "ObjectTypeQuery3" :!type "EObjectTypeQuery Enum") :`DrawTime` 2.0))
  (for _array_element _outhits
    (bind _asbp_enemy (cast `/Game/Main/BluePrints/BP_Enemy` (`.HitActor` (`GameplayStatics.BreakHitResult` _array_element))))
    (`KismetArrayLibrary.Array_AddUnique` (`self.TargetEnemies`) _asbp_enemy)))

(fn `GetWeapon_CanMove`
  (returns (CanMove :type Boolean))
  (return (`self.CanMove`)))

(fn `GetWeapon_Combat`
  (returns (Combat :type "/Game/Main/Character/ECombatType Enum"))
  (return (`self.Combat`)))

(fn `GetWeapon_Current`
  (returns (Weapon :type "/Game/Main/BP_Weapon Object Reference"))
  (return (`self.Sword`)))

(fn `GetWeapon_State`
  (returns (`State ` :type "/Game/Main/Character/Boss/AI/Pieta_Sword/EStateType Enum"))
  (return (`self.State`)))

(fn `PlayPlayerMontage`
  (bind (_montage _playerrate _startsectionname _canmove) (break `/Game/FCombo_Player_Montage` (`|GetArrayItem` (`self.ComboMontages`) (`/Game/Main/BluePrints/BP_Sword.ComboCount` (`self.Sword`)))))
  (`self.PlayAnimMontage` _montage _playerrate _startsectionname)
  (`/Game/Main/BP_Weapon.SetCanMove` (`self.Sword`) _canmove))

(fn `SetTargetCursor`
  (params (Enemy :type "/Game/Main/BluePrints/BP_Enemy Object Reference"))
  (for _array_element (`self.TargetEnemies`)
    (if (== _array_element (`local.Enemy`))
      (bind _lockcursor (`/Game/Main/BluePrints/BP_Enemy.LockCursor` _array_element))
      (`SceneComponent.SetVisibility` _lockcursor true false)
      (else
        (`SceneComponent.SetVisibility` _lockcursor false false)))))

(fn `SetWeapon_CanMove`
  (params (CanMove :type Boolean))
  (returns (Result :type Boolean))
  (bind _output_get (set `self.CanMove` CanMove))
  (return _output_get))

(fn `SetWeapon_Combat`
  (params (Combat :type "/Game/Main/Character/ECombatType Enum" :default "NewEnumerator0"))
  (returns (Result :type "/Game/Main/Character/ECombatType Enum"))
  (set `self.Combat` Combat)
  (return "NewEnumerator0"))

(fn `SetWeapon_State`
  (params (State :type "/Game/Main/Character/Boss/AI/Pieta_Sword/EStateType Enum" :default "NewEnumerator0"))
  (returns (Result :type "/Game/Main/Character/Boss/AI/Pieta_Sword/EStateType Enum"))
  (set `self.State` State)
  (return "NewEnumerator0"))

(fn `UserConstructionScript`)

(fn `Weapon_Change`
  (params (NewWeapon :type "/Game/Main/BP_Weapon Object Reference"))
  (returns (Weapon :type "/Game/Main/BP_Weapon Object Reference"))
  (return null))

(fn `Weapon_Dead`
  (returns (Result :type Boolean))
  (`PrimitiveComponent.SetCollisionEnabled` (`self.CapsuleComponent`) "NoCollision")
  (`self.K2_DestroyActor` (`self.Sword`))
  (`self.K2_DestroyActor`)
  (return false))

(fn `Weapon_Hitted`
  (returns (Result :type Boolean))
  (bind _weapon (`self.Weapon`)
    (:`then`
      (`/Game/Main/BP_Weapon.End Attack` _weapon)
      (return false))
    (:`else`)))