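; Sword weapon for the Pieta enemy, running its melee and second-phase attacks and a laser attack.
; Capsule overlaps send damage, with collision off at BeginPlay and toggled by events.
; Attack starts montages by combat type; EndAttack advances per-type combo counters, replaying montages until each limit resets.
; LaserAttack activates projectile movement, hides the sword and calls the enemy's laser; sword-rain and sphere-trace hit logic are disconnected.
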(event `SetWeaponCharacter`
  (params (Character :type "/Game/Main/BluePrints/BP_Enemy Object Reference"))
  (set `self.Enemy` Character))

(event `self.ReceiveBeginPlay`
  (`|ExecutionSequence`
    (:`then_0`
      (`self.SetOffCollision`))))

(event `self.Capsule.OnComponentBeginOverlap`
  (params (OverlappedComponent :type "PrimitiveComponent Object Reference") (OtherActor :type "Actor Object Reference") (OtherComp :type "PrimitiveComponent Object Reference") (OtherBodyIndex :type Integer) (bFromSweep :type Boolean) (SweepResult :type "HitResult Structure (by ref)"))
  (`self.SendDamage` OtherActor))

(event `OffCollision`
  ;[1 1 1] Collision
  (`PrimitiveComponent.SetCollisionEnabled` (`self.Capsule`) "NoCollision"))

(event `self.SetOnCollision`
  ;[1 1 1] Collision
  (`PrimitiveComponent.SetCollisionEnabled` (`self.Capsule`) "QueryAndPhysics"))

(event `SetOffCollision`
  ;[1 1 1] Collision
  (`PrimitiveComponent.SetCollisionEnabled` (`self.Capsule`) "NoCollision"))

(event `self.Attack`
  ;[1 1 1] 코멘트
  (`/Engine/EditorBlueprintResources/StandardMacros.IsValid` (`/Game/Main/BluePrints/BP_Enemy.Weapon` (`self.Enemy`))
    (:`Is Valid`
      (switch `/Game/Main/Character/ECombatType` (`self.GetCombat`)
        (:`NewEnumerator2`
          (`self.SetCanMove` false)
          (`/Game/Main/BluePrints/BP_Enemy.PlayPietaMontage` (`self.Enemy`)))
        (:`NewEnumerator6`
          (`self.SetCanMove` false)
          (`/Game/Main/BluePrints/BP_Enemy.Play2PhaseAttack` (`self.Enemy`)))))))

(event `self.End Attack`
  ;[1 1 1] 코멘트
  (`parent.End Attack`)
  (switch `/Game/Main/Character/ECombatType` (`/Game/Main/BluePrints/BP_Enemy.Combat` (`self.Enemy`))
    (:`NewEnumerator2`
      (if (>= (`self.PietaComboCount`) 2)
        (set `self.PietaComboCount` 0)
        (`self.SetCanMove` true)
        (else
          (`/Engine/EditorBlueprintResources/StandardMacros.IncrementInt` (`self.PietaComboCount`)
            (:`  `
              (`/Game/Main/BluePrints/BP_Enemy.PlayPietaMontage` (`self.Enemy`))
              (`self.SetCanMove` true))))))
    (:`NewEnumerator6`
      (if (>= (`self.Pieta2PhaseCount`) 5)
        (set `self.Pieta2PhaseCount` 3)
        (`self.SetCanMove` true)
        (else
          (`/Engine/EditorBlueprintResources/StandardMacros.IncrementInt` (`self.Pieta2PhaseCount`)
            (:`  `
              (`/Game/Main/BluePrints/BP_Enemy.PlayPietaMontage` (`self.Enemy`))
              (`self.SetCanMove` true))))))))

(event `PlayPietaNextCombo`
  ;[1 1 1] 코멘트
)

(fn `HittedPlayer`)

(fn `LaserAttack`
  (`ActorComponent.Activate` (`/Game/BP_LaserAttack.ProjectileMovement` (`self.Laser`)) false)
  (`self.SetActorHiddenInGame` true)
  (`/Game/Main/BluePrints/BP_Enemy.LaserAttack` (`self.Enemy`)))

(fn `SwordRainAttack`)

(fn `UserConstructionScript`)