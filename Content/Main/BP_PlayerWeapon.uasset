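; BP_PlayerWeapon is a player weapon Blueprint built for data-table-driven melee-style montage combos.
; PlayComboMontage plays the current combo entry's montage on the owning Character and applies its movement permission.
; Combo table loading, input buffering through EnableNextCombo/ExistNextCombo, and chaining logic are present but disconnected.
; BeginPlay, Attack and PlayNextCombp are empty, so nothing in this Blueprint triggers a combo.
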(event `self.ReceiveBeginPlay`
  ;[1 1 1] 몽타주 세팅
)

(event `self.Attack`
  ;[1 1 1] Attack
)

(event `PlayNextCombp`)

(fn `PlayComboMontage`
  (bind (_montage _playerrate _startsectionname _canmove) (break `/Game/FCombo_Player_Montage` (`|GetArrayItem` (`self.ComboMontages`) (`self.ComboCount`))))
  (bind `_as캐릭터` (cast `Character` (`self.GetOwner`)))
  (`Character.PlayAnimMontage` `_as캐릭터` _montage _playerrate _startsectionname) ; 캐릭터를 가져와야함
  (`self.SetCanMove` _canmove))

(fn `UserConstructionScript`)